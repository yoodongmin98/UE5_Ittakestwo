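; Laser beam effect actor that aims along its up vector at an attack position, or follows its spawn reference's rotation when no attack actor is set.
; Each Tick it reorients, box-traces forward and stretches the color-tinted mesh to the hit distance or maximum length.
; Without an attack actor, player hits leave beam length unchanged.
; GetHitActor exposes the hit actor; impact spawning and player damage are disconnected.
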(event EventBeginPlay
  (CallFunction|ChangeColor))

(event EventTick
  (params (DeltaSeconds :type Float%20%28single-precision%29))
  (if (Variables|Default|GetbAttackActor)
    (Variables|Default|SetMyRotation (Math|Rotator|MakeRotfromZ (- (Variables|Default|GetAttackActorPos) (Transformation|GetActorLocation))))
    (else
      (Variables|Default|SetMyRotation (Transformation|GetWorldRotation (Variables|/Script/Engine.Actor|GetRootComponent (Variables|Default|GetSpawnReference))))))
  (Variables|Default|SetEndvector (Transformation|GetActorUpVector))
  (Transformation|SetActorTransform (Math|Transform|MakeTransform (Transformation|GetWorldLocation (Variables|Default|GetArrow)) (Variables|Default|GetMyRotation) "1.000000,1.000000,1.000000"))
  (CallFunction|SetEndPoint))

(fn ConstructionScript
  (|CallParentFunction))

(fn ChangeColor
  (bind _returnvalue (Rendering|Material|CreateDynamicMaterialInstance (Variables|Default|GetSM_Parent) 0 "/Game/Map/FX/Laser/M_LaserFX.M_LaserFX" "None" :!class /Script/Engine.PrimitiveComponent))
  (Rendering|Material|SetVectorParameterValue _returnvalue "Color" (Variables|Default|GetLaserColor) :!class /Script/Engine.MaterialInstanceDynamic))

(fn SetEndPoint
  (bind _returnvalue (Transformation|GetActorLocation))
  (bind (_outhit _returnvalue_2) (Collision|BoxTraceByChannel _returnvalue (+ _returnvalue (* (Variables|Default|GetEndvector) (Variables|Default|GetRaserSize))) "0.500000,0.500000,0.500000" "0, 0, 0" "TraceTypeQuery3" false 0 "None" true "(R=0.000000,G=1.000000,B=1.000000,A=1.000000)" "(R=1.000000,G=0.000000,B=1.000000,A=1.000000)"))
  (if _returnvalue_2
    (bind _output_get (LocalVariables|SetLaserHitInfo _outhit))
    (bind _output_get_2 (Variables|Default|SetLocal%20Hit%20Actor (.HitActor (Collision|BreakHitResult _output_get))))
    (if (Variables|Default|GetbAttackActor)
      (Transformation|SetWorldScale3D (Variables|Default|GetSM_Parent) (Math|Vector|MakeVector 0.3 0.3 (Math|Float|SelectFloat (/ (+ (.Distance (Collision|BreakHitResult _output_get)) 1.0) 1e+02) (/ (Variables|Default|GetRaserSize) 1e+02) (.bBlockingHit (Collision|BreakHitResult _output_get)))) :!label _label)
      ;[1 1 1] 플레이어 체크 후 데미지 적용
      (if (Actor|ActorHasTag (Variables|Default|GetLocal%20Hit%20Actor) "Player")
        (bind _asplayer_base (Utilities|Casting|CastToPlayerBase (Variables|Default|GetLocal%20Hit%20Actor))))
      (elif (not (Actor|ActorHasTag _output_get_2 "Player"))
        (goto _label)))
    (else
      (Transformation|SetWorldScale3D (Variables|Default|GetSM_Parent) (Math|Vector|MakeVector 0.3 0.3 (/ (Variables|Default|GetRaserSize) 1e+02))))))

(fn GetHitActor
  (return (Variables|Default|GetLocal%20Hit%20Actor)))