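; Game state for a two-character (Cody and May) split-screen game that coordinates startup, local players and the start of play.
; BeginPlay shows a logo widget, then switches the game mode's default pawn to BP_FollowView after a delay.
; Events create local players, toggle splitscreen and update flags on all follow-view pawns.
; Replicated role selection triggers custom widget creation on both characters and the flying saucer, then tells GameManager the game has started.
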(event Custom|CreateLocalPlayer
  (Class|GameplayStatics|CreatePlayer -1)
  (Utilities|FlowControl|Delay 0.3)
  (bind _outactors (Actor|GetAllActorsOfClass "/Game/View/Blueprint/BP_FollowView.BP_FollowView_C"))
  (for _array_element _outactors
    (Variables|/Game/View/Blueprint/BP_FollowView.BP_FollowView_C|SetDoSetting _array_element true)))

(event Custom|SplitscreenMode
  (params (bDisable :type Boolean))
  (Class|GameplayStatics|SetForceDisableSplitscreen bDisable)
  (bind _outactors (Actor|GetAllActorsOfClass "/Game/View/Blueprint/BP_FollowView.BP_FollowView_C"))
  (for _array_element _outactors
    (Variables|/Game/View/Blueprint/BP_FollowView.BP_FollowView_C|SetIsCutscene _array_element bDisable)))

(event Custom|ResetScreen
  (bind _outactors (Actor|GetAllActorsOfClass "/Game/View/Blueprint/BP_FollowView.BP_FollowView_C"))
  (for _array_element _outactors
    (Variables|/Game/View/Blueprint/BP_FollowView.BP_FollowView_C|SetIsClientStop _array_element false)))

(event EventBeginPlay
  (bind _returnvalue (Game|GetGameMode))
  (bind _returnvalue_2 (UserInterface|CreateWidget "/Game/UI/Blueprint/WBP_Logo.WBP_Logo_C"))
  (UserInterface|Viewport|AddtoViewport _returnvalue_2 0)
  (Utilities|FlowControl|Delay 3.0)
  (Utilities|IsValid _returnvalue
    (:Is%20Valid
      (Variables|/Script/Engine.GameModeBase|SetDefaultPawnClass _returnvalue "/Game/View/Blueprint/BP_FollowView.BP_FollowView_C"))))

(event EventTick
  (params (DeltaSeconds :type Float%20%28single-precision%29)))

(fn ConstructionScript)

(fn OnRepIsRoleSelected
  (if (Variables|Default|GetIsRoleSelected)
    (bind _returnvalue (Actor|GetActorOfClass "/Game/Characters/Cody/BP/BP_Cody.BP_Cody_C"))
    (Utilities|IsValid _returnvalue
      (:Is%20Valid
        (Default|CreateAllCustomWidgets _returnvalue)
        (bind _returnvalue_2 (Actor|GetActorOfClass "/Game/Characters/May/BP/BP_May.BP_May_C"))
        (Utilities|IsValid _returnvalue_2
          (:Is%20Valid
            (Default|CreateAllCustomWidgets _returnvalue_2)
            (bind _returnvalue_3 (Actor|GetActorOfClass "/Game/Characters/EnemyFlyingSaucer/BluePrints/BP_EnemyFlyingSaucer.BP_EnemyFlyingSaucer_C"))
            (Utilities|IsValid _returnvalue_3
              (:Is%20Valid
                (Default|CreateAllCustomWidgets _returnvalue_3)
                (Variables|Default|SetReadyForPlay true)
                (bind _asgame_manager (Utilities|Casting|CastToGameManager (Game|GetGameInstance)))
                (Class|GameManager|SetGameStart _asgame_manager)))))))))