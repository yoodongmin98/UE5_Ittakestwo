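; Player character Blueprint for Cody, handling wall movement, health UI and death/respawn on top of inherited state getters.
; Tick runs trace-based wall slide, homing dismount and marker tinting, while jump input switches to a launched wall jump when sliding.
; Tick also mirrors HP and death state into variables whose OnRep handlers drive HUD materials, sounds, death effects and respawn teleport.
; The older DeathParticle path is disconnected.
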(event Custom|CreateAllCustomWidgets
  ;[1 1 1] Widget 생성
  (bind _returnvalue (UserInterface|CreateWidget "/Game/UI/Blueprint/WBP_CodyHpUI.WBP_CodyHpUI_C"))
  (UserInterface|Viewport|AddtoViewport _returnvalue 0)
  (Variables|Default|SetPlayerHpWidget _returnvalue)
  (bind _returnvalue_2 (UserInterface|CreateWidget "/Game/UI/Blueprint/WBP_Respawn.WBP_Respawn_C"))
  (UserInterface|Viewport|AddtoViewport _returnvalue_2 0)
  (bind _output_get (Variables|Default|SetRespawnUI _returnvalue_2))
  (Class|UserWidget|SetPositioninViewport _output_get "(X=320.000000,Y=0.000000)" true)
  (Widget|SetVisibility _output_get "Hidden"))

(event Custom|SetServerUIVisible
  ;[1 1 1] UIVisibleSetting
  (CallFunction|SetMultiUIVisible))

(event Custom|JumpEvent
  ;[1 1 1] Jump Event
  (CallFunction|WallJumpFunction))

(event Custom|SetMultiUIVisible
  (bind _playerhpwidget (Variables|Default|GetPlayerHpWidget))
  (bind _respawnui (Variables|Default|GetRespawnUI))
  (bind _playerhpwidget_2 (Variables|Default|GetPlayerHpWidget))
  (bind _respawnui_2 (Variables|Default|GetRespawnUI))
  ;[1 1 1] UIVisibleSetting
  (if (Class|PlayerBase|GetIsPlayerDeath)
    (Utilities|IsValid _playerhpwidget
      (:Is%20Valid
        (Widget|SetVisibility _playerhpwidget "Hidden")
        (Utilities|IsValid _respawnui
          (:Is%20Valid
            (Widget|SetVisibility _respawnui "Visible")))))
    (else
      (Utilities|IsValid _playerhpwidget_2
        (:Is%20Valid
          (Widget|SetVisibility _playerhpwidget_2 "Visible")
          (Utilities|IsValid _respawnui_2
            (:Is%20Valid
              (Widget|SetVisibility _respawnui_2 "Hidden"))))))))

(event Input|EnhancedActionEvents|EnhancedInputActionIA_Jump
  (params (ActionValue :type Boolean) (ElapsedSeconds :type Float%20%28double-precision%29) (TriggeredSeconds :type Float%20%28double-precision%29) (InputAction :type Input%20Action%20Object%20Reference :default "/Game/Characters/Cody/BP/Input/IA_Jump.IA_Jump"))
  ;[1 1 1] Jump Event
  (:Started
    (if (Variables|Default|GetbIsWallSlide)
      (CallFunction|JumpEvent)
      (else
        (Character|Jump))))
  (:Completed
    (Character|StopJumping)))

(event EventBeginPlay
  (bind _markeruiwidget (Variables|Default|GetMarkerUIWidget))
  (bind _markerinstance (Variables|/Script/UE5_ITT.MarkerWidget|GetMarkerInstance _markeruiwidget))
  ;[1 1 1] BeginPlay
  (CallFunction|ImpotController,Widget)
  (Utilities|FlowControl|Delay 1e+01)
  (if (not (Variables|Default|GetIsSetWidgetColor))
    (Utilities|IsValid _markerinstance
      (:Is%20Valid
        (bind _aswbp_marker_indicator (Utilities|Casting|CastToWBP_MarkerIndicator _markerinstance))
        (Variables|/Script/UMG.UserWidget|SetColorAndOpacity _aswbp_marker_indicator "(R=0.000000,G=0.170543,B=0.854167,A=1.000000)")
        (Variables|Default|SetIsSetWidgetColor true)))))

(event EventTick
  (params (DeltaSeconds :type Float%20%28single-precision%29))
  (bind _markeruiwidget (Variables|Default|GetMarkerUIWidget))
  (bind _markerinstance (Variables|/Script/UE5_ITT.MarkerWidget|GetMarkerInstance _markeruiwidget))
  ;[1 1 1] Event Tick
  (CallFunction|WallSlideFunction)
  (CallFunction|PlayerHpFunction)
  (CallFunction|GetOffHoming)
  (if (not (Variables|Default|GetIsSetWidgetColor))
    (Utilities|IsValid _markerinstance
      (:Is%20Valid
        (bind _aswbp_marker_indicator (Utilities|Casting|CastToWBP_MarkerIndicator _markerinstance))
        (Variables|/Script/UMG.UserWidget|SetColorAndOpacity _aswbp_marker_indicator "(R=0.000000,G=0.170543,B=0.854167,A=1.000000)")
        (Variables|Default|SetIsSetWidgetColor true)))))

(event Input|KeyboardEvents|F9
  (params (Key :type Key%20Structure :default "None"))
  ;[1 1 1] Test Attack
  (:Pressed
    (Class|PlayerBase|AttackPlayer 12)))

(fn ConstructionScript)

(fn WallSlideFunction
  (bind _returnvalue (Transformation|GetActorLocation))
  (bind _charactermovement (Variables|Character|GetCharacterMovement))
  (if (AI|Components|NavMovement|IsFalling (Variables|Character|GetCharacterMovement))
    (bind (_outhit _returnvalue_2) (Collision|LineTraceByChannel _returnvalue (+ _returnvalue (* (Transformation|GetActorForwardVector) 5.0)) "TraceTypeQuery1" false 0 "None"))
    (if _returnvalue_2
      (Variables|Default|SetbIsWallSlide true)
      (Transformation|SetActorRotation (Math|Rotator|MakeRotator 0.0 0.0 (+ (.yaw (Math|Conversions|RotationFromXVector (.ImpactNormal (Collision|BreakHitResult _outhit)))) 1.8e+02)))
      (Variables|/Script/Engine.MovementComponent|SetVelocity _charactermovement (Math|Interpolation|VInterptoConstant (Variables|/Script/Engine.MovementComponent|GetVelocity _charactermovement) "0, 0, 0" (Utilities|Time|GetWorldDeltaSeconds) 2e+03))
      (else
        (Variables|Default|SetbIsWallSlide false)))))

(fn ImpotController,Widget
  (bind _as플레이어_컨트롤러 (Utilities|Casting|CastToPlayerController (Pawn|GetController)))
  (Input|AddMappingContext (PlayerController|LocalPlayerSubsystems|GetEnhancedInputLocalPlayerSubsystem _as플레이어_컨트롤러) "/Game/Characters/Cody/BP/Input/IMC_Cody.IMC_Cody" 0 "(bIgnoreAllPressedKeysUntilRelease=True,bForceImmediately=False,bNotifyUserSettings=False)")
  (Variables|Default|SetPlayerHpUI (Class|PlayerBase|GetPlayerHP))
  (Variables|Default|SetIsDeathNotify (Class|PlayerBase|GetIsPlayerDeath)))

(fn PlayerHpFunction
  (if (== (Class|PlayerBase|GetPlayerHP) (Variables|Default|GetPlayerHpUI))
    _
    (else
      (Variables|Default|SetPlayerHpUI (Class|PlayerBase|GetPlayerHP))))
  (if (not (== (Class|PlayerBase|GetIsPlayerDeath) (Variables|Default|GetIsDeathNotify)))
    (Variables|Default|SetIsDeathNotify (Class|PlayerBase|GetIsPlayerDeath))))

(fn WallJumpFunction
  (Transformation|SetActorRotation (Math|Rotator|MakeRotator 0.0 0.0 (+ (.yaw (Transformation|GetActorRotation)) 1.8e+02)))
  (Character|LaunchCharacter (+ (* (Transformation|GetActorForwardVector) 1.5e+02) (Math|Vector|MakeVector 0.0 0.0 (Variables|/Script/Engine.CharacterMovementComponent|GetJumpZVelocity (Variables|Character|GetCharacterMovement)))) true true))

(fn GetOffHoming
  (if (Class|PlayerBase|GetOverlapHoming)
    (Class|PlayerBase|SetFlyFalse)
    (Character|LaunchCharacter (+ (* (* (Transformation|GetActorForwardVector) "-1.000000,-1.000000,-1.000000") 5e+02) (Math|Vector|MakeVector 0.0 0.0 (Variables|/Script/Engine.CharacterMovementComponent|GetJumpZVelocity (Variables|Character|GetCharacterMovement)))) true true)
    (Class|PlayerBase|SetOverlapHoming)
    (Class|PlayerBase|SpringArmDefaultFunction)))

(fn CutSceneAnimation
  (if (Class|Cody|GetCutScenceTrigger)
    (Components|Animation|PlayAnimation (Variables|Character|GetMesh) "/Game/Characters/Cody/Animation/Behaviour/PlayRoom/CutScene/PlayRoom_SpaceStation_BossFight_LaserRippedOff_Cody_Anim1.PlayRoom_SpaceStation_BossFight_LaserRippedOff_Cody_Anim1" false)))

(fn DeathParticle
  (if (Class|PlayerBase|GetIsPlayerDeath)
    (Pawn|Components|CharacterMovement|DisableMovement (Variables|Character|GetCharacterMovement))
    (if (Variables|Default|GetDeath%20Bool)
      (if (not (Rendering|IsVisible (Variables|Character|GetMesh)))
        (if (== (Class|PlayerBase|GetPlayerHP) (Class|PlayerBase|GetPlayerFullHP))
          (if (not (Variables|Default|GetResPawnBool))
            (Variables|Default|SetResPawnBool true)
            (Class|Cody|SetCodyMoveable)
            (Class|PlayerBase|SetRespawnPosition)
            (Rendering|SetVisibility (Variables|Character|GetMesh) true false)
            (Variables|Default|SetDeath%20Bool false)
            (bind _returnvalue (Class|PlayerBase|GetResPawnPosition))
            (Transformation|Teleport _returnvalue "0, 0, 0")
            (Collision|SetActorEnableCollision true))))
      (else
        (AddComponent|AddNiagaraComponent false (Math|Transform|MakeTransform (+ (Math|Vector|GetUpVector (Variables|Character|GetMesh)) "0.000000,0.000000,150.000000") "0, 0, 0" "1.000000,1.000000,1.000000"))
        (Variables|Default|SetDeath%20Bool true)
        (Rendering|SetVisibility (Variables|Character|GetMesh) false false)
        (Class|PlayerBase|SetCodyHoldEnemyTrue)
        (Collision|SetActorEnableCollision false) ; 되는건지 안되는건지 모름 ㄹㅇ
        (Variables|Default|SetResPawnBool false)))))

(fn OnRepPlayerHpUI
  (if (Class|PlayerBase|GetIsPlayerDeath)
    (CallFunction|RespawnUIAnimation)
    (else
      (CallFunction|HPUIAnimation))))

(fn HPUIAnimation
  (bind _playerhpwidget (Variables|Default|GetPlayerHpWidget))
  (Utilities|IsValid _playerhpwidget
    (:Is%20Valid
      (bind _returnvalue (Appearance|GetDynamicMaterial (Variables|/Game/UI/Blueprint/WBP_CodyHpUI.WBP_CodyHpUI_C|GetwbPlayerHpImage _playerhpwidget) :!class /Script/UMG.Image))
      (Rendering|Material|SetScalarParameterValue _returnvalue "bHpParameter" (/ (Math|Conversions|ToFloat(Integer) (Class|PlayerBase|GetPlayerHP)) (Class|PlayerBase|GetPlayerFullHP)) :!class /Script/Engine.MaterialInstanceDynamic)
      (Default|AttackEvent (Variables|Default|GetPlayerHpWidget)))))

(fn RespawnUIAnimation
  (bind _respawnui (Variables|Default|GetRespawnUI))
  (Utilities|IsValid _respawnui
    (:Is%20Valid
      (bind _returnvalue (Appearance|GetDynamicMaterial (Variables|/Game/UI/Blueprint/WBP_Respawn.WBP_Respawn_C|GetwbRespawnGage _respawnui) :!class /Script/UMG.Image))
      (Rendering|Material|SetScalarParameterValue _returnvalue "RespawnParamter" (/ (Math|Conversions|ToFloat(Integer) (Class|PlayerBase|GetPlayerHP)) (Class|PlayerBase|GetPlayerFullHP)) :!class /Script/Engine.MaterialInstanceDynamic)
      (Default|PressRespawn _respawnui))))

(fn OnRepIsDeathNotify
  (bind _respawnui (Variables|Default|GetRespawnUI))
  (bind _playerhpwidget (Variables|Default|GetPlayerHpWidget))
  (bind _respawnui_2 (Variables|Default|GetRespawnUI))
  (bind _playerhpwidget_2 (Variables|Default|GetPlayerHpWidget))
  (if (Variables|Default|GetIsDeathNotify)
    (Utilities|IsValid _playerhpwidget
      (:Is%20Valid
        (Widget|SetVisibility _playerhpwidget "Hidden")
        (Utilities|IsValid _respawnui_2
          (:Is%20Valid
            (Widget|SetVisibility _respawnui_2 "Visible")
            (CallFunction|RespawnUIAnimation)
            (Audio|PlaySound2D "/Game/Sound/UI/SoundCue/SC_GameOverOnePlayer.SC_GameOverOnePlayer" 1.0 1.0 0.0 0 0)
            (Audio|PlaySound2D "/Game/Sound/UI/SoundCue/SC_ReSpawnHeartAppear.SC_ReSpawnHeartAppear" 1.0 1.0 0.0 0 0)
            (Utilities|IsValid (Variables|Default|GetLoopSound)
              (:Is%20Valid
                _)
              (:Is%20Not%20Valid
                (bind _returnvalue (Audio|SpawnSound2D "/Game/Sound/UI/SoundCue/SC_HealthReSpawnLoop.SC_HealthReSpawnLoop" 1.0 1.0 0.0 0))
                (bind _output_get (Variables|Default|SetLoopSound _returnvalue))))
            (Components|Activation|SetActive (Variables|Default|GetLoopSound) true false)
            (Pawn|Components|CharacterMovement|DisableMovement (Variables|Character|GetCharacterMovement))
            (Niagara|SpawnSystematLocation "/Game/Characters/Cody/CodyDeathParticle.CodyDeathParticle" (+ (Transformation|GetWorldLocation (Variables|Character|GetMesh)) "0.000000,0.000000,150.000000"))
            (Rendering|SetVisibility (Variables|Character|GetMesh) false false)
            (Collision|SetActorEnableCollision false) ; 되는건지 안되는건지 모름 ㄹㅇ
          ))))
    (else
      (Utilities|IsValid _playerhpwidget_2
        (:Is%20Valid
          (Widget|SetVisibility _playerhpwidget_2 "Visible")
          (Utilities|IsValid _respawnui
            (:Is%20Valid
              (Widget|SetVisibility _respawnui "Hidden")
              (CallFunction|HPUIAnimation)
              (Audio|PlaySound2D "/Game/Sound/UI/SoundCue/SC_HealthBarFullHealth.SC_HealthBarFullHealth" 1.0 1.0 0.0 0 0)
              (Utilities|IsValid (Variables|Default|GetLoopSound)
                (:Is%20Valid
                  (Components|Activation|SetActive (Variables|Default|GetLoopSound) false false)
                  (Class|PlayerBase|SetRespawnPosition)
                  (Rendering|SetVisibility (Variables|Character|GetMesh) true false)
                  (bind _returnvalue_2 (Class|PlayerBase|GetResPawnPosition))
                  (Transformation|Teleport _returnvalue_2 "0, 0, 0")
                  (Collision|SetActorEnableCollision true))))))))))