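; Lobby player pawn for two-player role selection, where host and client each pick Cody or May.
; Left/Right moves a player's choice, blocking a role the other holds, with host and remote input split by authority and RepNotifies driving WBP_RoleSelectionUI animations.
; Enter locks the choice with a sound.
; Once both lock, it spawns and possesses the characters, flags the GameState, creates an extra local player, triggers BP_FollowView setup and destroys the selection pawns.
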(event Custom|ClientPressLeft
  ;[1 1 1] Character Selection
  (CallFunction|ReplicateEventUser2))

(event Custom|ClientPressRIght
  ;[1 1 1] Character Selection
  (CallFunction|ReplicateEventUser1))

(event Custom|ChangeUser2
  (params (role :type Integer))
  ;[1 1 1] Character Selection
  (switch int role
    (:1
      _)
    (:2
      _))
  (Variables|Default|SetChangeDone2 true)
  (bind _asbp_player_base (Utilities|Casting|CastToBP_PlayerBase (Game|Player|GetPlayerPawn 0)))
  (Variables|BP_PlayerBase_C|SetChangeDone2 _asbp_player_base true)
  (CallFunction|PossessRole))

(event Custom|PossessRole
  (if (Variables|Default|GetChangeDone%201)
    (if (Variables|Default|GetChangeDone2)
      (CallFunction|HideRoleSelectUI)
      (Utilities|FlowControl|Delay 1.0)
      (bind _asbp_ittgame_state_base (Utilities|Casting|CastToBP_ITTGameStateBase (Game|GetGameState)))
      (Variables|/Game/GameState/BluePrints/BP_ITTGameStateBase.BP_ITTGameStateBase_C|SetIsRoleSelected _asbp_ittgame_state_base true)
      (Utilities|FlowControl|Delay 0.3)
      (Variables|Default|SetDivViewFunc true)
      (Utilities|FlowControl|Delay 0.3)
      (bind _outactors (Actor|GetAllActorsOfClass "/Game/View/Blueprint/BP_FollowView.BP_FollowView_C"))
      (for _array_element _outactors
        (Variables|/Game/View/Blueprint/BP_FollowView.BP_FollowView_C|SetDoSetting _array_element true))
      (bind _outactors_2 (Actor|GetAllActorsOfClass "BP_PlayerBase_C"))
      (for _array_element_2 _outactors_2
        (Actor|DestroyActor _array_element_2)))))

(event EventBeginPlay
  (CallFunction|LlinkRoleSelectWidget))

(event Collision|EventActorBeginOverlap
  (params (OtherActor :type Actor%20Object%20Reference)))

(event EventTick
  (params (DeltaSeconds :type Float%20%28single-precision%29)))

(event Input|KeyboardEvents|DebugKeyNumPadNine
  (params (Key :type Key%20Structure :default "None") (ActionValue :type Input%20Action%20Value%20Structure))
  ;[1 1 1] Character Selection
  (:Pressed
    (Utilities|IsValid (Variables|Default|GetWidget%20UI)
      (:Is%20Valid
        (Variables|Default|SetView%20Widget%20UI (not (Variables|Default|GetView%20Widget%20UI)))))))

(event Input|KeyboardEvents|Left
  (params (Key :type Key%20Structure :default "None"))
  ;[1 1 1] Character Selection
  (:Pressed
    (Utilities|IsValid (Variables|Default|GetWidget%20UI)
      (:Is%20Valid
        (CallFunction|SelectLeft)))))

(event Input|KeyboardEvents|Right
  (params (Key :type Key%20Structure :default "None"))
  ;[1 1 1] Character Selection
  (:Pressed
    (Utilities|IsValid (Variables|Default|GetWidget%20UI)
      (:Is%20Valid
        (CallFunction|SelectRight)))))

(event Input|KeyboardEvents|Enter
  (params (Key :type Key%20Structure :default "None"))
  ;[1 1 1] Character Selection
  (:Pressed
    (Networking|SwitchHasAuthority
      (:Authority
        (CallFunction|ChangeUser1))
      (:Remote
        (CallFunction|ChangeUser2 (Variables|Default|GetCurUser2))))))

(fn ConstructionScript)

(fn SelectLeft
  (Networking|SwitchHasAuthority
    (:Authority
      (if (not (Variables|Default|GetChangeDone%201))
        (switch int (Variables|Default|GetCur%20User%201)
          (:0
            (bind _asbp_player_base (Utilities|Casting|CastToBP_PlayerBase (Game|Player|GetPlayerPawn 1)))
            (if (!= 2 (Variables|BP_PlayerBase_C|GetCurUser2 _asbp_player_base))
              (Variables|Default|SetNextUser1 2)))
          (:1
            (Variables|Default|SetNextUser1 0)))))
    (:Remote
      (if (not (Variables|Default|GetChangeDone2))
        (CallFunction|ClientPressLeft)))))

(fn SelectRight
  (Networking|SwitchHasAuthority
    (:Authority
      (if (not (Variables|Default|GetChangeDone%201))
        (switch int (Variables|Default|GetCur%20User%201)
          (:0
            (bind _asbp_player_base (Utilities|Casting|CastToBP_PlayerBase (Game|Player|GetPlayerPawn 1)))
            (if (!= 1 (Variables|BP_PlayerBase_C|GetCurUser2 _asbp_player_base))
              (Variables|Default|SetNextUser1 1)))
          (:2
            (Variables|Default|SetNextUser1 0)))))
    (:Remote
      (if (not (Variables|Default|GetChangeDone2))
        (CallFunction|ClientPressRIght)))))

(fn ReplicateEventUser2
  (switch int (Variables|Default|GetCurUser2)
    (:0
      (bind _asbp_player_base (Utilities|Casting|CastToBP_PlayerBase (Game|Player|GetPlayerPawn 0)))
      (if (!= 2 (Variables|BP_PlayerBase_C|GetCur%20User%201 _asbp_player_base))
        (Variables|Default|SetNextUser2 2)))
    (:1
      (Variables|Default|SetNextUser2 0))))

(fn ReplicateEventUser1
  (switch int (Variables|Default|GetCurUser2)
    (:0
      (bind _asbp_player_base (Utilities|Casting|CastToBP_PlayerBase (Game|Player|GetPlayerPawn 0)))
      (if (!= 1 (Variables|BP_PlayerBase_C|GetCur%20User%201 _asbp_player_base))
        (Variables|Default|SetNextUser2 1)))
    (:2
      (Variables|Default|SetNextUser2 0))))

(fn OnRepNextUser1
  (bind _widget_ui (Variables|Default|GetWidget%20UI))
  (if (Utilities|IsValid _widget_ui)
    (Default|MainUIAnimation _widget_ui (Variables|Default|GetCur%20User%201) (Variables|Default|GetNextUser1) true)
    (Variables|Default|SetCur%20User%201 (Variables|Default|GetNextUser1))))

(fn OnRepNextUser2
  (bind _widget_ui (Variables|Default|GetWidget%20UI))
  (Networking|SwitchHasAuthority
    (:Authority
      (Default|MainUIAnimation (Variables|Default|GetWidget%20UI) (Variables|Default|GetCurUser2) (Variables|Default|GetNextUser2) false)
      (Variables|Default|SetCurUser2 (Variables|Default|GetNextUser2)))
    (:Remote
      (Utilities|IsValid _widget_ui
        (:Is%20Valid
          (Default|MainUIAnimation _widget_ui (Variables|Default|GetCurUser2) (Variables|Default|GetNextUser2) false)
          (Variables|Default|SetCurUser2 (Variables|Default|GetNextUser2)))))))

(fn ChangeUser1
  (switch int (Variables|Default|GetCur%20User%201)
    (:1
      _)
    (:2
      _))
  (Variables|Default|SetChangeDone%201 true)
  (bind _asbp_player_base (Utilities|Casting|CastToBP_PlayerBase (Game|Player|GetPlayerPawn 1)))
  (Variables|BP_PlayerBase_C|SetChangeDone%201 _asbp_player_base true)
  (CallFunction|PossessRole))

(fn PossessFunc
  (bind _returnvalue (Game|GetPlayerController 0))
  (bind _returnvalue_2 (Game|GetPlayerController 1))
  (Game|SpawnActorfromClass "/Game/Characters/Cody/BP/BP_Cody.BP_Cody_C" (Math|Transform|MakeTransform "180.000000,-3900.000000,150.000000" "0, 0, 0" "1.000000,1.000000,1.000000") "Undefined" "MultiplyWithRoot" 0 0)
  (Game|SpawnActorfromClass "/Game/Characters/May/BP/BP_May.BP_May_C" (Math|Transform|MakeTransform "-180.000000,-3900.000000,150.000000" "0, 0, 0" "1.000000,1.000000,1.000000") "Undefined" "MultiplyWithRoot" 0 0)
  (bind _asbp_player_base (Utilities|Casting|CastToBP_PlayerBase (Game|Player|GetPlayerPawn 0)))
  (switch int (Variables|BP_PlayerBase_C|GetCur%20User%201 _asbp_player_base)
    (:1
      (bind _returnvalue_3 (Actor|GetActorOfClass "/Game/Characters/Cody/BP/BP_Cody.BP_Cody_C"))
      (Pawn|Possess _returnvalue _returnvalue_3))
    (:2
      (bind _returnvalue_4 (Actor|GetActorOfClass "/Game/Characters/May/BP/BP_May.BP_May_C"))
      (Pawn|Possess _returnvalue _returnvalue_4)))
  (bind _asbp_player_base_2 (Utilities|Casting|CastToBP_PlayerBase (Game|Player|GetPlayerPawn 1)))
  (switch int (Variables|BP_PlayerBase_C|GetCurUser2 _asbp_player_base_2)
    (:1
      (bind _returnvalue_5 (Actor|GetActorOfClass "/Game/Characters/Cody/BP/BP_Cody.BP_Cody_C"))
      (Pawn|Possess _returnvalue_2 _returnvalue_5))
    (:2
      (bind _returnvalue_6 (Actor|GetActorOfClass "/Game/Characters/May/BP/BP_May.BP_May_C"))
      (Pawn|Possess _returnvalue_2 _returnvalue_6))))

(fn OnRepViewWidgetUI
  (Utilities|IsValid (Variables|Default|GetWidget%20UI)
    (:Is%20Valid
      (if (Variables|Default|GetView%20Widget%20UI)
        (Widget|SetVisibility (Variables|Default|GetWidget%20UI) "Visible")
        (else
          (Widget|SetVisibility (Variables|Default|GetWidget%20UI) "Hidden"))))))

(fn LlinkRoleSelectWidget
  (bind _asbp_ittgame_state_base (Utilities|Casting|CastToBP_ITTGameStateBase (Game|GetGameState)))
  (if (not (Variables|/Game/GameState/BluePrints/BP_ITTGameStateBase.BP_ITTGameStateBase_C|GetIsRoleSelected _asbp_ittgame_state_base))
    (bind _foundwidgets (Widget|GetAllWidgetsOfClass "/Game/UI/Blueprint/WBP_RoleSelectionUI.WBP_RoleSelectionUI_C" true))
    (Utilities|IsValid (Utilities|Array|Get(acopy) _foundwidgets)
      (:Is%20Valid
        (bind _output_get (Variables|Default|SetWidget%20UI (Utilities|Array|Get(acopy) _foundwidgets)))
        (Widget|SetVisibility _output_get "Visible")
        (Variables|Default|SetView%20Widget%20UI true)))))

(fn OnRepDivViewFunc
  (Class|GameplayStatics|CreatePlayer -1))

(fn HideRoleSelectUI
  (Variables|Default|SetView%20Widget%20UI false)
  (CallFunction|PossessFunc)
  (bind _returnvalue (Actor|GetActorOfClass "/Game/UI/StartLevel/RoseArm/BP_Rose_Arm.BP_Rose_Arm_C"))
  (Actor|DestroyActor _returnvalue))

(fn OnRepChangeDone2
  (if (== (Variables|Default|GetCurUser2) 1)
    (Audio|PlaySound2D "/Game/Sound/UI/SoundCue/SC_CodySelect.SC_CodySelect" 1.0 1.0 0.0 0 0)
    (else
      (Audio|PlaySound2D "/Game/Sound/UI/SoundCue/SC_MaySelect.SC_MaySelect" 1.0 1.0 0.0 0 0))))

(fn OnRepChangeDone1
  (if (== (Variables|Default|GetCur%20User%201) 1)
    (Audio|PlaySound2D "/Game/Sound/UI/SoundCue/SC_CodySelect.SC_CodySelect" 1.0 1.0 0.0 0 0)
    (else
      (Audio|PlaySound2D "/Game/Sound/UI/SoundCue/SC_MaySelect.SC_MaySelect" 1.0 1.0 0.0 0 0))))