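; BP_FollowView is a camera actor that manages player views for the Cody and May co-op characters.
; Outside cutscenes, once DoSetting is true, Tick branches on authority, and the server assigns view targets among player controllers once.
; Clients find the partner character and snap ViewCameraComponent to its controller transform every tick, with the Cody client also swapping view targets once.
; An IsCutscene RepNotify re-arms that one-time assignment when a cutscene starts.
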(event EventBeginPlay
  (Transformation|SetActorTransform (Math|Transform|MakeTransform "950.000000,-9000.000000,3000.000000" "0, 0, 0" "1.000000,1.000000,1.000000")))

(event Collision|EventActorBeginOverlap
  (params (OtherActor :type Actor%20Object%20Reference)))

(event EventTick
  (params (DeltaSeconds :type Float%20%28single-precision%29))
  (if (not (Variables|Default|GetIsCutscene))
    (if (Variables|Default|GetDoSetting)
      (Networking|SwitchHasAuthority
        (:Authority
          (CallFunction|ServerViewFunc))
        (:Remote
          (Utilities|IsValid (Variables|Default|GetTargetActor)
            (:Is%20Valid
              (CallFunction|ClientViewFunc))
            (:Is%20Not%20Valid
              (CallFunction|SetClientTarget))))))))

(fn ConstructionScript)

(fn ServerViewFunc
  (if (not (Variables|Default|GetIsClientStop))
    (if (Actor|ActorHasTag (Game|Player|GetPlayerPawn 0) "Cody")
      (Game|Player|SetViewTargetwithBlend (Game|GetPlayerController 0) (Game|GetPlayerController 2) 0.0 "VTBlend_Linear" 0.0 false)
      (Game|Player|SetViewTargetwithBlend (Game|GetPlayerController 1) (Game|GetPlayerController 0) 0.0 "VTBlend_Linear" 0.0 false)
      (else
        (Game|Player|SetViewTargetwithBlend (Game|GetPlayerController 1) (Game|GetPlayerController 2) 0.0 "VTBlend_Linear" 0.0 false)))
    (Variables|Default|SetIsClientStop true)))

(fn SetClientTarget
  (if (Actor|ActorHasTag (Game|Player|GetPlayerPawn 0) "May")
    (bind _returnvalue (Actor|GetActorOfClass "/Game/Characters/Cody/BP/BP_Cody.BP_Cody_C"))
    (Utilities|IsValid _returnvalue
      (:Is%20Valid
        (Variables|Default|SetTargetActor _returnvalue)
        (Variables|Default|SetIsCody true)))
    (elif (Actor|ActorHasTag (Game|Player|GetPlayerPawn 0) "Cody")
      (bind _returnvalue_2 (Actor|GetActorOfClass "/Game/Characters/May/BP/BP_May.BP_May_C"))
      (Utilities|IsValid _returnvalue_2
        (:Is%20Valid
          (Variables|Default|SetTargetActor _returnvalue_2)
          (Variables|Default|SetIsCody false))))))

(fn SetTargetCamTrans
  (bind _targetactor (Variables|Default|GetTargetActor))
  (bind _view_camera_component (Variables|Default|GetView%20Camera%20Component))
  (Transformation|SetWorldRotation _view_camera_component (Class|PlayerBase|GetCurControllerRot _targetactor) false false)
  (Transformation|SetWorldLocation _view_camera_component (Class|PlayerBase|GetCurControllerLoc _targetactor) false true))

(fn ClientViewFunc
  (if (Actor|ActorHasTag (Game|Player|GetPlayerPawn 0) "Cody")
    (if (Variables|Default|GetIsClientStop)
      (CallFunction|SetTargetCamTrans)
      (else
        (Game|Player|SetViewTargetwithBlend (Game|GetPlayerController 1) (Game|GetPlayerController 0) 0.0 "VTBlend_Linear" 0.0 false)
        (Game|Player|SetViewTargetwithBlend (Game|GetPlayerController 0) (Game|GetPlayerController 1) 0.0 "VTBlend_Linear" 0.0 false)
        (Variables|Default|SetIsClientStop true)
        (CallFunction|SetTargetCamTrans)))
    (else
      (CallFunction|SetTargetCamTrans))))

(fn OnRepIsCutscene
  (if (Variables|Default|GetIsCutscene)
    (Variables|Default|SetIsClientStop false)))